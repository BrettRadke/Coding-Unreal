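; BP_SpawnManager runs enemy waves in the level, spawning the first one shortly after BeginPlay.
; SpawnEnemies finds every BP_SpawnPoint and spawns a BP_Enemy at each one's root transform.
; NewWaveCheck, which comments say dying enemies call, counts BP_Enemy actors and respawns a wave after a delay when one or none remain.
; Debug strings are printed throughout to trace the flow.
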(event `self.ReceiveBeginPlay`
  (`KismetSystemLibrary.PrintString` "Spawn Mangaer Exists.") ; Tell the player that we exist
  (`KismetSystemLibrary.Delay` 1.0) ; wait for some time
  (`self.Spawn Enemies`) ; call the Spawn Enemies event
)

(event `Spawn Enemies`
  (bind _outactors (`GameplayStatics.GetAllActorsOfClass` "/Game/Blueprints/BP_SpawnPoint.BP_SpawnPoint_C")) ; get an array of all spawn points on a level
  (for _array_element _outactors
    (`KismetSystemLibrary.PrintString` (`KismetSystemLibrary.GetDisplayName` _array_element) true true (struct :`R` 1.0 :`G` 0.148993 :`A` 1.0) 10.0) ; print the name
    (`|SpawnActorFromClass` "/Game/Blueprints/BP_Enemy.BP_Enemy_C" (`SceneComponent.K2_GetComponentToWorld` (`/Game/Blueprints/BP_SpawnPoint.DefaultSceneRoot` _array_element)) "Undefined" "MultiplyWithRoot" null null) ; Spawn Actor from class BP_Enemy
  )
  (`KismetSystemLibrary.PrintString` "Finished with the For Each Loop for spawn enemies"))

(event `NewWaveCheck`
  (`KismetSystemLibrary.PrintString` "Was that the last enemy?")
  (bind _outactors (`GameplayStatics.GetAllActorsOfClass` "/Game/Blueprints/BP_Enemy.BP_Enemy_C")) ; get an array of all BP enemies in a level
  (bind _returnvalue (`KismetArrayLibrary.Array_Length` _outactors))
  (`KismetSystemLibrary.PrintString` (`KismetStringLibrary.Concat_StrStr` "There are" (`KismetStringLibrary.Conv_IntToString` _returnvalue) "enemies in the level") true true (struct :`R` 0.003605 :`G` 1.0 :`A` 1.0))
  (if (> _returnvalue 1)
    (`KismetSystemLibrary.PrintString` "You are not the last one") ; It's not time for new enemies yet
    (else
      (`KismetSystemLibrary.PrintString` "New Wave incoming!" true true (struct :`R` 1.0 :`B` 0.001649 :`A` 1.0))
      (`KismetSystemLibrary.Delay` 3.0)
      (`self.Spawn Enemies`) ; Spawn Enemies Again
    )))

(fn `UserConstructionScript`)