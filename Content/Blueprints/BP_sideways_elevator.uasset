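; Sideways elevator actor that moves its Cube platform when the player presses a key inside a trigger box.
; Overlapping BoxElevator prints a "go forward" prompt and enables player input, which is disabled on exit, with no check on the overlapping actor.
; Q flip-flops a timeline forward and back, setting the Cube's relative location.
; E drives a second timeline the same way for going down, noted as unfinished.
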(event `self.Box elevator.OnComponentBeginOverlap`
  (params (OverlappedComponent :type "PrimitiveComponent Object Reference") (OtherActor :type "Actor Object Reference") (OtherComp :type "PrimitiveComponent Object Reference") (OtherBodyIndex :type Integer) (bFromSweep :type Boolean) (SweepResult :type "HitResult Structure (by ref)"))
  ;[0 0.2959 1 0.5] elevator controlls
  ;;[1 0 0.03592 0.5] going up!
  (`KismetSystemLibrary.PrintString` "Press \"Q\" to go forward!" true true (struct :`R` 0.467951 :`G` 0.362346 :`B` 1.0 :`A` 1.0))
  (`self.EnableInput` (`GameplayStatics.GetPlayerController` 0)))

(event `self.Box elevator.OnComponentEndOverlap`
  (params (OverlappedComponent :type "PrimitiveComponent Object Reference") (OtherActor :type "Actor Object Reference") (OtherComp :type "PrimitiveComponent Object Reference") (OtherBodyIndex :type Integer))
  ;[0 0.2959 1 0.5] elevator controlls
  ;;[1 0 0.03592 0.5] going up!
  (`self.DisableInput` (`GameplayStatics.GetPlayerController` 0)))

(event `Key|Q`
  (params (Key :type "Key Structure"))
  ;[0 0.2959 1 0.5] elevator controlls
  ;;[1 0 0.03592 0.5] going up!
  (:`Pressed`
    (`/Engine/EditorBlueprintResources/StandardMacros.FlipFlop`
      (:`A`
        (bind (_direction _elevator_going_up_) (`Timeline|Timeline` :!label _label)
          (:`Update`
            (`SceneComponent.K2_SetRelativeLocation` (`self.Cube`) _elevator_going_up_ false false))))
      (:`B`
        (goto _label :!via `Reverse`)))))

(event `Key|E`
  (params (Key :type "Key Structure"))
  ;[0 0.2959 1 0.5] elevator controlls
  ;;[0 1 0.2085 0.5] elevator going down not completed!
  (:`Pressed`
    (`/Engine/EditorBlueprintResources/StandardMacros.FlipFlop`
      (:`A`
        (bind (_direction _elevator_going_down_) (`Timeline|Timeline_0` :!label _label_2)
          (:`Update`
            (`SceneComponent.K2_SetRelativeLocation` (`self.Cube`) _elevator_going_down_ false false))))
      (:`B`
        (goto _label_2 :!via `Reverse`)))))

(fn `UserConstructionScript`)