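; Falling platform that drops a short time after the player character steps into its trigger, then returns to its start.
; An IsReady flag gates a chain of custom events: Activated waits a configurable delay, Falling turns on physics, and Resetting follows three seconds later.
; Resetting turns physics off and uses a timeline to lerp from the fallen transform back to the one saved at BeginPlay.
; Each state swaps the platform material.
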(event `self.ReceiveBeginPlay`
  ;[0 0.01917 0.15 0.5] begin fall
  (set `self.Original Transform` (`SceneComponent.K2_GetComponentToWorld` (`self.Platform`))) ; recording start location and location
  (`PrimitiveComponent.SetMaterial` (`self.Platform`) 0 "/Game/Materials/PlatformMaterials/MI_PLatform_Ready.MI_PLatform_Ready"))

(event `self.Box Trigger.OnComponentBeginOverlap`
  (params (OverlappedComponent :type "PrimitiveComponent Object Reference") (OtherActor :type "Actor Object Reference") (OtherComp :type "PrimitiveComponent Object Reference") (OtherBodyIndex :type Integer) (bFromSweep :type Boolean) (SweepResult :type "HitResult Structure (by ref)"))
  ;[0.15 0.1168 0 0.5] beginning part
  (`KismetSystemLibrary.PrintString` "somehting ran into my trigger!!!")
  (if (`self.isReady`)
    (cast `/Game/Blueprints/BP_ThirdPersonCharacter1` OtherActor)
    (`self.Activated`)))

(event `Activated`
  ;[0.15 0.01877 0 0.5] activation
  (`KismetSystemLibrary.PrintString` "Activated!")
  (`PrimitiveComponent.SetMaterial` (`self.Platform`) 0 "/Game/Materials/PlatformMaterials/MI_Platform_Activated.MI_Platform_Activated")
  (set `self.isReady` false) ; WE ARE NOT READY
  (`KismetSystemLibrary.Delay` (`self.Fall Delay Duration`))
  (`self.Falling`))

(event `Falling`
  ;[0 0.15 0.01761 0.5] falling
  (`KismetSystemLibrary.PrintString` "falling")
  (`PrimitiveComponent.SetMaterial` (`self.Platform`) 0 "/Game/Materials/PlatformMaterials/MI_Platform_Falling.MI_Platform_Falling")
  (`PrimitiveComponent.SetSimulatePhysics` (`self.Platform`) true)
  (`KismetSystemLibrary.Delay` 3.0)
  (`self.Resetting`))

(event `Resetting`
  ;[0.05012 0 0.15 0.5] resetting
  (`KismetSystemLibrary.PrintString` "Resetting now!")
  (`PrimitiveComponent.SetMaterial` (`self.Platform`) 0 "/Game/Materials/PlatformMaterials/MI_Platform_Resetting.MI_Platform_Resetting")
  (set `self.Fallen Transform` (`SceneComponent.K2_GetComponentToWorld` (`self.Platform`)))
  (`PrimitiveComponent.SetSimulatePhysics` (`self.Platform`) false)
  (bind (_direction _newtrack_0) (`Timeline|returntostart` :!via `PlayFromStart`)
    (:`Update`
      (bind (_returnvalue_location _returnvalue_rotation) (`KismetMathLibrary.BreakTransform` (`KismetMathLibrary.TLerp` (`self.Fallen Transform`) (`self.Original Transform`) _newtrack_0)))
      (`SceneComponent.K2_SetWorldLocationAndRotation` (`self.Platform`) _returnvalue_location _returnvalue_rotation false false))
    (:`Finished`
      (set `self.isReady` true) ; WE ARE READY NOW!
      (`PrimitiveComponent.SetMaterial` (`self.Platform`) 0 "/Game/Materials/PlatformMaterials/MI_PLatform_Ready.MI_PLatform_Ready"))))

(fn `UserConstructionScript`)